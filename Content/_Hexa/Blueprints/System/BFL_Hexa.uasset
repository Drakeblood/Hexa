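; Blueprint function library of shared accessors for the Hexa game's core objects and heroes.
; It returns the game mode and game instance already cast to GM_Hexa and BP_GameInstance.
; Hero lookups read the game mode's Players array, either fetching one hero by index or averaging all their actor locations into a center point, with no empty-array guard.
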(fn GetHexaGameMode
  (return (.AsGM%20Hexa (Utilities|Casting|CastToGM_Hexa (Game|GetGameMode)))))

(fn GetHexaGameInstance
  (return (.AsBP%20Game%20Instance (Utilities|Casting|CastToBP_GameInstance (Game|GetGameInstance)))))

(fn GetHero
  (params (Index :type Integer))
  (return (Utilities|Array|Get(acopy) (Variables|/Game/_Hexa/Blueprints/GM_Hexa.GM_Hexa_C|GetPlayers (CallFunction|GetHexaGameMode)) Index)))

(fn GetAverageHeroesLocation
  (bind _hexagamemode (CallFunction|GetHexaGameMode))
  (bind _players (Variables|/Game/_Hexa/Blueprints/GM_Hexa.GM_Hexa_C|GetPlayers _hexagamemode))
  (for _array_element _players
    (LocalVariables|SetLocationsSum (+ (Transformation|GetActorLocation _array_element) (LocalVariables|GetLocationsSum))))
  (return (/ (LocalVariables|GetLocationsSum) (Utilities|Array|Length _players))))