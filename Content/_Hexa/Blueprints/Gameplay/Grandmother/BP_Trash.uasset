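; BP_Trash is a physics-driven trash actor for the Grandmother gameplay that drifts around in random horizontal directions.
; On BeginPlay it picks a direction and starts a looping timer, with a randomly chosen interval, to pick new ones.
; Tick applies an impulse to the static mesh along that direction, with strength randomized around Force by ForceDeviation.
; An alternative AddForce call is left unconnected.
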(event Custom|ChangeRandomDirection
  (bind _returnvalue (Math|Random|RandomUnitVector))
  (Variables|Default|SetRandomDirection (Math|Vector|MakeVector (.x _returnvalue) (.y _returnvalue) 0.0)))

(event EventTick
  (params (DeltaSeconds :type Float%20%28single-precision%29))
  (bind _forcedeviation (Variables|Default|GetForceDeviation))
  (Physics|AddImpulse (Variables|Default|GetStaticMesh) (* (Variables|Default|GetRandomDirection) (+ (Variables|Default|GetForce) (Math|Random|RandomFloatinRange (* _forcedeviation -1.0) _forcedeviation))) "None" false))

(event EventBeginPlay
  (Utilities|Time|SetTimerbyEvent (delegate Custom|ChangeRandomDirection) (Math|Random|RandomFloatinRange 1.5 3.0) true)
  (CallFunction|ChangeRandomDirection))

(fn ConstructionScript)