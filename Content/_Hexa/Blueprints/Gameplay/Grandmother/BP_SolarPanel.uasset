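; BP_SolarPanel is a pickup in the Grandmother gameplay that the picking hero equips on pickup.
; If the other hero carries a vacuum cleaner and stands too far away, that hero plays a move toward the picker.
; When that movement timeline ends, a bound event asks the Hexa game mode to add a rope between the players.
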(event Custom|Light)

(event Custom|OnGoNextToSecondHeroTimelineEnd_Event
  (Default|AddRopetoPlayers (CallFunction|GetHexaGameMode)))

(event EventOnPickup
  (params (Hero :type BP%20Hero%20Character%20Object%20Reference))
  (bind _hero (CallFunction|GetSecondHero Hero))
  (Default|EquipSolarPanel Hero self)
  (Utilities|IsValid (Variables|/Game/_Hexa/Blueprints/Character/BP_HeroCharacter.BP_HeroCharacter_C|GetVacuumCleaner _hero)
    (:Is%20Valid
      (if (> (Transformation|GetDistanceTo _hero Hero) 6e+02)
        (EventDispatchers|AssignOnGoNexttoSecondHeroTimelineEnd _hero (delegate Custom|OnGoNextToSecondHeroTimelineEnd_Event))
        (Default|PlayGoNexttoSecondHero _hero)))))

(fn ConstructionScript)