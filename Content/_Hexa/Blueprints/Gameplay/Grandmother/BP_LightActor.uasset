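; BP_LightActor is a directional light emitter that powers BP_SolarPanel actors where its beam lands.
; Each Tick it line traces 1000 units along its Arrow component's forward vector.
; On a hit, it runs a Radius-sized sphere overlap at the impact location and calls Light on every solar panel found.
; A debug sphere draw for that area is present but disconnected.
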(event EventTick
  (params (DeltaSeconds :type Float%20%28single-precision%29))
  (bind _arrow (Variables|Default|GetArrow))
  (bind _returnvalue (Transformation|GetWorldLocation _arrow))
  (bind (_outhit _returnvalue_2) (Collision|LineTraceByChannel _returnvalue (+ _returnvalue (* (Math|Vector|GetForwardVector _arrow) 1e+03)) "TraceTypeQuery4" false 0 "None"))
  (if _returnvalue_2
    (bind _outactors (Collision|SphereOverlapActors (.location _outhit) (Variables|Default|GetRadius) (Utilities|Array|MakeArray "ObjectTypeQuery2") "/Game/_Hexa/Blueprints/Gameplay/Grandmother/BP_SolarPanel.BP_SolarPanel_C"))
    (for _array_element _outactors
      (Default|Light (.AsBP%20Solar%20Panel (Utilities|Casting|CastToBP_SolarPanel _array_element))))))

(fn ConstructionScript)