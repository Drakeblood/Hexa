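; BP_LightPath moves a referenced light actor along a spline as a guiding path, looping while the BP_NPC quest is playing.
; PlayTimeline unhides the light and runs a timeline that places it by spline distance, keeping its initial height offset from the path actor.
; Play rate derives from Duration, re-randomized within DurationDeviation on every update.
; When a pass finishes, it replays if QuestPlaying is set, otherwise hides the light.
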(event Custom|PlayTimeline
  (bind _durationdeviation (Variables|Default|GetDurationDeviation))
  (Rendering|SetActorHiddenInGame (Variables|Default|GetLightActor) false)
  (bind _newtrack_0 (Timeline|MoveAroundSplineTimeline PlayFromStart)
    (:Update
      (Components|Timeline|SetPlayRate (Variables|Default|GetMoveAroundSplineTimeline) (/ 1.0 (+ (Variables|Default|GetDuration) (Math|Random|RandomFloatinRange (* _durationdeviation -1.0) _durationdeviation))))
      (Transformation|SetActorLocation (Variables|Default|GetLightActor) (+ (Spline|GetLocationatDistanceAlongSpline (Variables|Default|GetSpline) (Math|Float|Lerp 0.0 (Spline|GetDistanceAlongSplineatSplinePoint (Variables|Default|GetSpline) (- (Spline|GetNumberOfSplinePoints (Variables|Default|GetSpline)) 1)) _newtrack_0) "World") (Math|Vector|MakeVector 0.0 0.0 (.z (Variables|Default|GetLightActorOffset)))) false false))
    (:Finished
      (bind _returnvalue (Actor|GetActorOfClass "/Game/_Hexa/Blueprints/Character/BP_NPC.BP_NPC_C"))
      (if (Variables|/Game/_Hexa/Blueprints/Character/BP_NPC.BP_NPC_C|GetQuestPlaying _returnvalue)
        (CallFunction|PlayTimeline)
        (else
          (Rendering|SetActorHiddenInGame (Variables|Default|GetLightActor) true))))))

(fn ConstructionScript
  (Components|Timeline|SetPlayRate (Variables|Default|GetMoveAroundSplineTimeline) (/ 1.0 (Variables|Default|GetDuration)))
  (bind _lightactor (Variables|Default|GetLightActor)
    (:then
      (Variables|Default|SetLightActorOffset (- (Transformation|GetActorLocation _lightactor) (Transformation|GetActorLocation))))
    (:else)))