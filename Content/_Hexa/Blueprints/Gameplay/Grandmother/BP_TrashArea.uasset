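; Trash area actor in the Grandmother gameplay that fills a box volume with scattered, scaled-down BP_Trash actors.
; FillArea starts a looping timer that spawns one randomly placed and rotated piece per tick, stores it in Trashes, and clears itself at TrashCount.
; CheckTrashes scans for a still-valid piece and sets EmptyTable true on finding one, despite the name, but its final branch does nothing.
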(event Custom|FillArea
  (bind _returnvalue (Utilities|Time|SetTimerbyEvent (delegate Custom|SpawnTrash) (Variables|Default|GetDelayBetweenSpawn) true)))

(event Custom|SpawnTrash
  (bind _box (Variables|Default|GetBox))
  (bind _returnvalue (Game|SpawnActorfromClass "/Game/_Hexa/Blueprints/Gameplay/Grandmother/BP_Trash.BP_Trash_C" (Math|Transform|MakeTransform (+ (Math|Random|RandomPointinBoundingBox (Transformation|GetWorldLocation _box) (Variables|/Script/Engine.BoxComponent|GetBoxExtent _box)) (Variables|Default|GetSpawnOffset)) (Math|Random|RandomRotator true) "0.100000,0.100000,0.100000") "AlwaysSpawn" "MultiplyWithRoot" 0 0))
  (bind _returnvalue_2 (Utilities|Array|Add (Variables|Default|GetTrashes) _returnvalue))
  (if (== _returnvalue_2 (- (Variables|Default|GetTrashCount) 1))
    (Utilities|Time|ClearandInvalidateTimerbyHandle (stale Custom|FillArea _returnvalue))))

(fn ConstructionScript)

(fn CheckTrashes
  (bind _array_element (Utilities|Array|ForEachLoopwithBreak (Variables|Default|GetTrashes) :!label _label)
    (:LoopBody
      (if (Utilities|IsValid _array_element)
        (LocalVariables|SetEmptyTable (Utilities|IsValid _array_element))
        (goto _label Break)))
    (:Completed
      (if (LocalVariables|GetEmptyTable)
        _))))