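; BP_VacuumCleaner is a vacuum cleaner pickup that a hero equips and uses to clear trash.
; On pickup, if the other hero has a solar panel, the game mode ropes the players together, first moving that hero over via a timeline if too far away.
; Clear sphere-overlaps BP_Trash around the attached hero's clear point, starting each one's death timeline and setting a short lifespan.
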(event Custom|Clear
  (bind _outactors (Collision|SphereOverlapActors (Transformation|GetWorldLocation (Variables|/Game/_Hexa/Blueprints/Character/BP_HeroCharacter.BP_HeroCharacter_C|GetVacuumCleanerClearSpherePoint (.AsBP%20Hero%20Character (Utilities|Casting|CastToBP_HeroCharacter (Actor|GetAttachParentActor))))) (Variables|Default|GetSphereRadius) (Utilities|Array|MakeArray "ObjectTypeQuery4") "/Game/_Hexa/Blueprints/Gameplay/Grandmother/BP_Trash.BP_Trash_C"))
  (for _array_element _outactors
    (Actor|SetLifeSpan _array_element 0.5)
    (Components|Timeline|PlayfromStart (Variables|/Game/_Hexa/Blueprints/Gameplay/Grandmother/BP_Trash.BP_Trash_C|GetDeathTimeline (.AsBP%20Trash (Utilities|Casting|CastToBP_Trash _array_element))))))

(event Custom|OnGoNextToSecondHeroTimelineEnd_Event
  (Default|AddRopetoPlayers (CallFunction|GetHexaGameMode)))

(event EventOnPickup
  (params (Hero :type BP%20Hero%20Character%20Object%20Reference))
  (bind _hero (CallFunction|GetSecondHero Hero))
  (Default|EquipVacuumCleaner Hero self)
  (Utilities|IsValid (Variables|/Game/_Hexa/Blueprints/Character/BP_HeroCharacter.BP_HeroCharacter_C|GetSolarPanel _hero)
    (:Is%20Valid
      (if (> (Transformation|GetDistanceTo _hero Hero) 6e+02)
        (EventDispatchers|AssignOnGoNexttoSecondHeroTimelineEnd _hero (delegate Custom|OnGoNextToSecondHeroTimelineEnd_Event))
        (Default|PlayGoNexttoSecondHero _hero)
        (else
          (Default|AddRopetoPlayers (CallFunction|GetHexaGameMode)))))))

(fn ConstructionScript)