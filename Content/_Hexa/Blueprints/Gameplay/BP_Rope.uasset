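; BP_Rope is the tether between the heroes, apparently limiting their separation to a maximum cable length.
; Each tick it places two spheres on either side of the heroes' average location, toward each player at half the cable length plus a collision offset, likely as moving barriers.
; A timed event temporarily sets a hero's IgnoreMovement flag.
; An unconnected graph holds older logic that pulls the other hero when the cable is taut.
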(event Custom|IgnoreMovementForHeroForTime
  (params (Hero :type BP%20Hero%20Character%20Object%20Reference) (Duration :type Float%20%28double-precision%29))
  (Variables|/Game/_Hexa/Blueprints/Character/BP_HeroCharacter.BP_HeroCharacter_C|SetIgnoreMovement Hero true)
  (Utilities|FlowControl|Delay Duration)
  (Variables|/Game/_Hexa/Blueprints/Character/BP_HeroCharacter.BP_HeroCharacter_C|SetIgnoreMovement Hero false))

(event EventTick
  (params (DeltaSeconds :type Float%20%28single-precision%29))
  (bind _returnvalue (CallFunction|GetAverageHeroesLocation))
  (for (_array_element _array_index) (Variables|/Game/_Hexa/Blueprints/GM_Hexa.GM_Hexa_C|GetPlayers (CallFunction|GetHexaGameMode))
    (Transformation|SetWorldLocation (Utilities|Array|Get(acopy) (Utilities|Array|MakeArray (Variables|Default|GetSphere1) (Variables|Default|GetSphere2)) _array_index) (+ _returnvalue (* (Math|Vector|GetForwardVector (Math|Rotator|FindLookatRotation _returnvalue (Transformation|GetActorLocation _array_element))) (+ (/ (Variables|Default|GetMaxCableLength) 2.0) (Variables|Default|GetCollisionOffset)))) false false)))

(fn ConstructionScript)