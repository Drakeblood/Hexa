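; BP_LightActor is a light source actor that lights up solar panels around the spot it points at.
; Every Tick it line traces forward from its Arrow component and, on a hit, runs a sphere overlap of Radius at the impact location.
; It calls Light on each BP_SolarPanel found and draws a debug sphere showing the affected area.
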(event EventTick
  (params (DeltaSeconds :type Float%20%28single-precision%29))
  (bind _arrow (Variables|Default|GetArrow))
  (bind _radius (Variables|Default|GetRadius))
  (bind _returnvalue (Transformation|GetWorldLocation _arrow))
  (bind (_outhit _returnvalue_2) (Collision|LineTraceByChannel _returnvalue (+ _returnvalue (* (Math|Vector|GetForwardVector _arrow) 1e+03)) "TraceTypeQuery4" false 0 "None"))
  (if _returnvalue_2
    (bind _outactors (Collision|SphereOverlapActors (.location _outhit) _radius (Utilities|Array|MakeArray "ObjectTypeQuery1" "ObjectTypeQuery2") "/Game/_Hexa/Blueprints/Gameplay/BP_SolarPanel.BP_SolarPanel_C"))
    (Rendering|Debug|DrawDebugSphere (.location _outhit) _radius 12 "(R=1.000000,G=1.000000,B=1.000000,A=1.000000)" 0.2 1.0)
    (for _array_element _outactors
      (Default|Light (.AsBP%20Solar%20Panel (Utilities|Casting|CastToBP_SolarPanel _array_element))))))

(fn ConstructionScript)