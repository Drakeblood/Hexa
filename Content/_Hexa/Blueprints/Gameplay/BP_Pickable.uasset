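; BP_Pickable is a world pickup that the hero can interact with, using a mesh set at construction.
; Interacting spawns an actor of the configured ItemClass far below the origin, sends it OnPickupMessage with the hero, then destroys the pickable.
; Focus events show and hide an interaction widget, and CanInteract always allows interaction.
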(event EventFocusBegin
  (params (Hero :type BP%20Hero%20Character%20Object%20Reference))
  (Rendering|SetVisibility (Variables|Default|GetInteractionWidget) true false))

(event EventFocusEnd
  (params (Hero :type BP%20Hero%20Character%20Object%20Reference))
  (Rendering|SetVisibility (Variables|Default|GetInteractionWidget) false false))

(event EventInteract
  (params (Hero :type BP%20Hero%20Character%20Object%20Reference))
  (bind _returnvalue (Game|SpawnActorfromClass (Variables|Default|GetItemClass) (Math|Transform|MakeTransform "0.000000,0.000000,-1000.000000" "0, 0, 0" "1.000000,1.000000,1.000000") "AlwaysSpawn" "MultiplyWithRoot" 0 0))
  (Class|BPIPickable|OnPickup(Message) _returnvalue Hero)
  (Actor|DestroyActor))

(fn ConstructionScript
  (Components|StaticMesh|SetStaticMesh (Variables|Default|GetStaticMesh) (Variables|Default|GetMesh)))

(fn CanInteract
  (params (Caller :type BP%20Hero%20Character%20Object%20Reference))
  (return true))