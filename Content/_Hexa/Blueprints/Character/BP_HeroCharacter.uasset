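; Playable hero character that registers with the game mode; the last one added takes the Lemoslaw mesh and animation, then signals that all players are valid.
; A per-tick sphere trace maintains the focused interactable through interface focus messages, which TryBeginInteract then triggers and clears.
; A timeline slides the hero beside the second hero, then fires and unbinds a one-shot end dispatcher.
; Equip functions snap a vacuum cleaner or solar panel to ToolSocket.
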(event Custom|TryBeginInteract
  (bind _currentinteractable (Variables|Interaction|GetCurrentInteractable)
    (:then
      (Class|BPIInteractable|Interact(Message) _currentinteractable self)
      (Class|BPIInteractable|FocusEnd(Message) _currentinteractable self)
      (Variables|Interaction|SetCurrentInteractable 0))
    (:else)))

(event Custom|PlayGoNextToSecondHero
  (bind _self self)
  (bind _hero (CallFunction|GetSecondHero _self))
  (Variables|Default|SetInitialLocation (Transformation|GetActorLocation))
  (bind _newtrack_0 (Timeline|GoNextToSecondHero PlayFromStart)
    (:Update
      (Transformation|SetActorLocation (Math|Vector|Lerp(Vector) (Variables|Default|GetInitialLocation) (+ (Transformation|GetActorLocation _hero) (* (Transformation|GetActorRightVector _hero) 1e+02)) _newtrack_0) false false))
    (:Finished
      (Default|CallOnGoNexttoSecondHeroTimelineEnd)
      (EventDispatchers|UnbindallEventsfromOnGoNexttoSecondHeroTimelineEnd))))

(event EventBeginPlay
  (bind _mesh (Variables|Character|GetMesh))
  (bind _returnvalue (Utilities|Array|Add (Variables|/Game/_Hexa/Blueprints/GM_Hexa.GM_Hexa_C|GetPlayers (CallFunction|GetHexaGameMode)) self))
  (if (== _returnvalue (- (Variables|/Game/_Hexa/Blueprints/System/BP_GameInstance.BP_GameInstance_C|GetPlayersNum (.AsBP%20Game%20Instance (Utilities|Casting|CastToBP_GameInstance (Game|GetGameInstance)))) 1))
    (Components|SkeletalMesh|SetSkeletalMeshAsset _mesh "/Game/_Hexa/Character/Lemoslaw/Lemoslaw_rig_animacje.Lemoslaw_rig_animacje")
    (Class|SkeletalMeshComponent|SetAnimClass _mesh "/Game/_Hexa/Character/Lemoslaw/ABP_Lemoslaw.ABP_Lemoslaw_C")
    (Utilities|FlowControl|DelayUntilNextTick)
    (Default|AllPlayersValid (CallFunction|GetHexaGameMode))))

(event EventTick
  (params (DeltaSeconds :type Float%20%28single-precision%29))
  (bind _returnvalue (Transformation|GetActorLocation))
  (bind (_outhit _returnvalue_2) (Collision|SphereTraceByChannel _returnvalue (+ _returnvalue "0.000000,0.000000,1.000000") (Variables|Interaction|GetInteractionRadius) "TraceTypeQuery3" false 0 "None" true "(R=1.000000,G=0.000000,B=0.000000,A=1.000000)" "(R=0.000000,G=1.000000,B=0.000000,A=1.000000)" 0.2))
  (if _returnvalue_2
    (bind _caninteract (Class|BPIInteractable|CanInteract(Message) (.hitactor _outhit) self))
    (if _caninteract
      (bind _currentinteractable (Variables|Interaction|GetCurrentInteractable)
        (:then
          (Class|BPIInteractable|FocusEnd(Message) _currentinteractable self))
        (:else
          _))
      (bind _output_get (Variables|Interaction|SetCurrentInteractable (.hitactor _outhit)))
      (Class|BPIInteractable|FocusBegin(Message) _output_get self)
      (else
        (bind _currentinteractable_2 (Variables|Interaction|GetCurrentInteractable :!label _label)
          (:then
            (Class|BPIInteractable|FocusEnd(Message) _currentinteractable_2 self)
            (Variables|Interaction|SetCurrentInteractable 0))
          (:else))))
    (else
      (goto _label))))

(fn ConstructionScript)

(fn EquipVacuumCleaner
  (params (VacuumCleaner :type BP%20Vacuum%20Cleaner%20Object%20Reference))
  (bind _output_get (Variables|Default|SetVacuumCleaner VacuumCleaner))
  (bind _returnvalue (Transformation|AttachComponentToComponent (Variables|/Script/Engine.Actor|GetRootComponent _output_get) (Variables|Character|GetMesh) "ToolSocket" "SnapToTarget" "SnapToTarget" "SnapToTarget" true))
  (Variables|Default|SetEquipped _returnvalue))

(fn EquipSolarPanel
  (params (SolarPanel :type BP%20Solar%20Panel%20Object%20Reference))
  (bind _output_get (Variables|Default|SetSolarPanel SolarPanel))
  (bind _returnvalue (Transformation|AttachComponentToComponent (Variables|/Script/Engine.Actor|GetRootComponent _output_get) (Variables|Character|GetMesh) "ToolSocket" "SnapToTarget" "SnapToTarget" "SnapToTarget" true))
  (Variables|Default|SetEquipped _returnvalue))