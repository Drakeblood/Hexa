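; BP_NPC is an interactable character that shows an interaction widget on focus and opens a dialogue when used.
; Closing the dialogue starts a big countdown timer on the HUD, via event dispatchers bound on the player controller's HUD widget.
; When the countdown ends, it finds the trash area and light path actors by class, fills the area and plays the path's timeline.
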(event Custom|OnDialogueClosed_Event
  (bind _hexaplayercontroller (CallFunction|GetHexaPlayerController))
  (bind _wbphud (Variables|/Game/_Hexa/Blueprints/Player/BP_PlayerController.BP_PlayerController_C|GetWBPHUD _hexaplayercontroller))
  (EventDispatchers|AssignOnBIgTimerCountdownEnd _wbphud (delegate Custom|OnBIgTimerCountdownEnd_Event))
  (Default|RunBigTimer _wbphud 5.0))

(event Custom|OnBIgTimerCountdownEnd_Event
  (bind _returnvalue (Actor|GetActorOfClass "/Game/_Hexa/Blueprints/Gameplay/Grandmother/BP_TrashArea.BP_TrashArea_C"))
  (Default|FillArea _returnvalue)
  (bind _returnvalue_2 (Actor|GetActorOfClass "/Game/_Hexa/Blueprints/Gameplay/Grandmother/BP_LightPath.BP_LightPath_C"))
  (Default|PlayTimeline _returnvalue_2))

(event EventBeginPlay
  (|CallParentFunction) ; This node is disabled and will not be called.\nDrag off pins to build functionality.
)

(event Collision|EventActorBeginOverlap
  (params (OtherActor :type Actor%20Object%20Reference))
  (|CallParentFunction OtherActor) ; This node is disabled and will not be called.\nDrag off pins to build functionality.
)

(event EventTick
  (params (DeltaSeconds :type Float%20%28single-precision%29))
  (|CallParentFunction DeltaSeconds) ; This node is disabled and will not be called.\nDrag off pins to build functionality.
)

(event EventFocusBegin
  (params (Hero :type BP%20Hero%20Character%20Object%20Reference))
  (Rendering|SetVisibility (Variables|Default|GetInteractionWidget) true false))

(event EventFocusEnd
  (params (Hero :type BP%20Hero%20Character%20Object%20Reference))
  (Rendering|SetVisibility (Variables|Default|GetInteractionWidget) false false))

(event EventInteract
  (params (Hero :type BP%20Hero%20Character%20Object%20Reference))
  (bind _hexaplayercontroller (CallFunction|GetHexaPlayerController))
  (bind _wbphud (Variables|/Game/_Hexa/Blueprints/Player/BP_PlayerController.BP_PlayerController_C|GetWBPHUD _hexaplayercontroller))
  (EventDispatchers|AssignOnDialogueClosed _wbphud (delegate Custom|OnDialogueClosed_Event))
  (Default|ShowDialogue _wbphud "help me cos tam smieci"))

(fn ConstructionScript
  (|CallParentFunction))

(fn CanInteract
  (params (Caller :type BP%20Hero%20Character%20Object%20Reference))
  (return true))