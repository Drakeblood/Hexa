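; Player controller that drives two heroes from a single controller, with separate Enhanced Input move and interact actions for each.
; Move applies input unless the hero ignores movement, projecting its position to screen space to block movement past a viewport edge margin.
; CheckMovementInputDuringRope, not called within this graph, pushes each hero toward the other while the other's move input is held.
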(event Input|EnhancedActionEvents|EnhancedInputActionIA_Move1
  (params (ActionValue :type Vector%202D%20Structure) (ElapsedSeconds :type Float%20%28double-precision%29) (TriggeredSeconds :type Float%20%28double-precision%29) (InputAction :type Input%20Action%20Object%20Reference :default "/Game/_Hexa/Input/IA_Move1.IA_Move1"))
  (bind _hero (CallFunction|GetHero))
  (if (not (Variables|/Game/_Hexa/Blueprints/Character/BP_HeroCharacter.BP_HeroCharacter_C|GetIgnoreMovement _hero))
    (CallFunction|Move ActionValue _hero)))

(event Input|EnhancedActionEvents|EnhancedInputActionIA_Move2
  (params (ActionValue :type Vector%202D%20Structure) (ElapsedSeconds :type Float%20%28double-precision%29) (TriggeredSeconds :type Float%20%28double-precision%29) (InputAction :type Input%20Action%20Object%20Reference :default "/Game/_Hexa/Input/IA_Move2.IA_Move2"))
  (bind _hero (CallFunction|GetHero 1))
  (if (not (Variables|/Game/_Hexa/Blueprints/Character/BP_HeroCharacter.BP_HeroCharacter_C|GetIgnoreMovement _hero))
    (CallFunction|Move ActionValue _hero)))

(event Input|EnhancedActionEvents|EnhancedInputActionIA_Interact1
  (params (ActionValue :type Boolean) (ElapsedSeconds :type Float%20%28double-precision%29) (TriggeredSeconds :type Float%20%28double-precision%29) (InputAction :type Input%20Action%20Object%20Reference :default "/Game/_Hexa/Input/IA_Interact1.IA_Interact1"))
  (:Started
    (Default|TryBeginInteract (CallFunction|GetHero))))

(event Input|EnhancedActionEvents|EnhancedInputActionIA_Interact2
  (params (ActionValue :type Boolean) (ElapsedSeconds :type Float%20%28double-precision%29) (TriggeredSeconds :type Float%20%28double-precision%29) (InputAction :type Input%20Action%20Object%20Reference :default "/Game/_Hexa/Input/IA_Interact2.IA_Interact2"))
  (:Started
    (Default|TryBeginInteract (CallFunction|GetHero 1))))

(event EventBeginPlay
  (bind _returnvalue (PlayerController|LocalPlayerSubsystems|GetEnhancedInputLocalPlayerSubsystem))
  (Utilities|IsValid _returnvalue
    (:Is%20Valid
      (Input|AddMappingContext _returnvalue "/Game/_Hexa/Input/IMC_Default.IMC_Default" 0 "(bIgnoreAllPressedKeysUntilRelease=True,bForceImmediately=False,bNotifyUserSettings=False)"))))

(fn ConstructionScript)

(fn Move
  (params (ActionValue :type Vector%202D%20Structure) (Hero :type BP%20Hero%20Character%20Object%20Reference))
  (bind _self self)
  (bind _self_2 self)
  (bind _returnvalue (Transformation|GetActorLocation Hero))
  (bind _returnvalue_2 (Transformation|GetActorLocation Hero))
  (bind _screenposition (Class|GameplayStatics|ProjectWorldtoScreen _self _returnvalue false))
  (bind _screenposition_2 (Class|GameplayStatics|ProjectWorldtoScreen _self_2 _returnvalue_2 false))
  (Utilities|FlowControl|Sequence
    (:then_0
      (if (or (and (> (.y _screenposition) 5e+01) (> (.y ActionValue) 0.0)) (and (< (.y _screenposition) (- (.SizeY (HUD|GetViewportSize)) 50)) (< (.y ActionValue) 0.0)))
        (Pawn|Input|AddMovementInput Hero (Math|Vector|GetForwardVector (Math|Rotator|MakeRotator 0.0 0.0 (.yaw (Pawn|GetControlRotation :!class /Script/Engine.Controller)))) (.y ActionValue) false)))
    (:then_1
      (if (or (and (> (.x _screenposition_2) 5e+01) (< (.x ActionValue) 0.0)) (and (< (.x _screenposition_2) (- (.SizeX (HUD|GetViewportSize)) 50)) (> (.x ActionValue) 0.0)))
        (Pawn|Input|AddMovementInput Hero (Math|Vector|GetRightVector (Math|Rotator|MakeRotator (.roll (Pawn|GetControlRotation :!class /Script/Engine.Controller)) 0.0 0.0)) (.x ActionValue) false)))))

(fn CheckMovementInputDuringRope
  (bind _hero (CallFunction|GetHero))
  (bind _hero_2 (CallFunction|GetHero 1))
  (Utilities|FlowControl|Sequence
    (:then_0
      (if (> (Math|Vector2D|Vector2DLength (Input|EnhancedActionValues|GetIA_Move1)) 0.0)
        (Pawn|Input|AddMovementInput _hero_2 (Math|Vector|GetForwardVector (Math|Rotator|FindLookatRotation (Transformation|GetActorLocation _hero_2) (Transformation|GetActorLocation (CallFunction|GetHero)))) 1.0 false)))
    (:then_1
      (if (> (Math|Vector2D|Vector2DLength (Input|EnhancedActionValues|GetIA_Move2)) 0.0)
        (Pawn|Input|AddMovementInput _hero (Math|Vector|GetForwardVector (Math|Rotator|FindLookatRotation (Transformation|GetActorLocation _hero) (Transformation|GetActorLocation (CallFunction|GetHero 1)))) 1.0 false)))))