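; GM_Hexa is the game mode that sets up local multiplayer and tracks a trash area quest.
; It creates an extra local player a tick after BeginPlay, with events to give all players a shared camera and link two heroes by rope.
; Trash score updates the first player's HUD, and quest end sets the state by a two-thirds threshold, then resets the score.
; AddValidPlayer's registration logic is unwired.
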(event Custom|AddRopeToPlayers
  (bind _returnvalue (Game|SpawnActorfromClass "/Game/_Hexa/Blueprints/Gameplay/Grandmother/BP_Rope.BP_Rope_C" (Math|Transform|MakeTransform "0, 0, 0" "0, 0, 0" "1.000000,1.000000,1.000000") "AlwaysSpawn" "MultiplyWithRoot" 0 0))
  (bind _output_get (Variables|Default|SetRope _returnvalue))
  (Transformation|AttachActorToActor _output_get (CallFunction|GetHero) "None" "SnapToTarget" "SnapToTarget" "SnapToTarget" true)
  (Class|CableComponent|SetAttachEndto (Variables|/Game/_Hexa/Blueprints/Gameplay/Grandmother/BP_Rope.BP_Rope_C|GetCable (Variables|Default|GetRope)) (CallFunction|GetHero 1) "None" "None")
  (Actor|Tick|SetActorTickEnabled (Variables|Default|GetRope) true))

(event Custom|AllPlayersValid
  (bind _returnvalue (Game|SpawnActorfromClass "/Game/_Hexa/Blueprints/Gameplay/BP_CommonCamera.BP_CommonCamera_C" (Math|Transform|MakeTransform (Transformation|GetActorLocation (Game|Player|GetPlayerPawn 0)) "0, 0, 0" "1.000000,1.000000,1.000000") "AlwaysSpawn" "MultiplyWithRoot" 0 0))
  (Variables|Default|SetCommonCamera _returnvalue)
  (for _array_element (Variables|Default|GetPlayers)
    (Game|Player|SetViewTargetwithBlend (.AsBP%20Player%20Controller (Utilities|Casting|CastToBP_PlayerController (Pawn|GetController _array_element))) (Variables|Default|GetCommonCamera) 0.0 "VTBlend_Linear" 0.0 false)))

(event EventBeginPlay
  (Utilities|FlowControl|DelayUntilNextTick)
  (Class|GameplayStatics|CreatePlayer -1))

(fn ConstructionScript)

(fn AddValidPlayer
  (params (Player :type BP%20Player%20State%20Object%20Reference%20%28by%20ref%29)))

(fn SetTrashAreaScore
  (params (TrashAreaScore :type Integer))
  (bind _output_get (Variables|Default|SetTrashAreaScore TrashAreaScore))
  (Variables|Default|GetTrashArea
    (:then
      _)
    (:else
      (bind _returnvalue (Actor|GetActorOfClass "/Game/_Hexa/Blueprints/Gameplay/Grandmother/BP_TrashArea.BP_TrashArea_C"))
      (bind _output_get_2 (Variables|Default|SetTrashArea _returnvalue))))
  (Rendering|Components|TextRender|SetText (Variables|/Game/_Hexa/Blueprints/UI/WBP_HUD.WBP_HUD_C|GetTrashesCountTextBlock (Variables|/Game/_Hexa/Blueprints/Player/BP_PlayerController.BP_PlayerController_C|GetWBPHUD (CallFunction|GetHexaPlayerController))) (Utilities|Text|FormatText "{Score}/{MaxScore}" _output_get (Variables|/Game/_Hexa/Blueprints/Gameplay/Grandmother/BP_TrashArea.BP_TrashArea_C|GetTrashCount _output_get_2))))

(fn OnEndTrashAreaQuest
  (Variables|Default|SetTrashAreaState (select (>= (Variables|Default|GetTrashAreaScore) (* (/ (Variables|/Game/_Hexa/Blueprints/Gameplay/Grandmother/BP_TrashArea.BP_TrashArea_C|GetTrashCount (Variables|Default|GetTrashArea)) 3) 2)) "NewEnumerator1" "NewEnumerator2"))
  (CallFunction|SetTrashAreaScore))